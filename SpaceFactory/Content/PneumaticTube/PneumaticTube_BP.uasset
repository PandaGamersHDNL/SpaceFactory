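; Pneumatic tube actor that lays pipe meshes along a spline as a chain of deformed spline mesh segments with collision.
; BuildSplineMesh runs from the construction script, and every Tick while BuildMode is on.
; It splits the spline into PipeLength steps, updating or creating a segment for each, with tangents clamped to that length to limit distortion.
; Surplus segments are destroyed when the spline shortens, and the component array is refilled from the spline's children.
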(event EventBeginPlay)

(event EventTick
  (params (DeltaSeconds :type Float%20%28single-precision%29))
  (if (Variables|Default|GetbBuildMode)
    (CallFunction|BuildSplineMesh)))

(fn ConstructionScript
  (CallFunction|BuildSplineMesh))

(fn BuildSplineMesh
  (bind _spline (Variables|Default|GetSpline))
  (bind _pipelength (Variables|Default|GetpipeLength))
  (bind _spline_2 (Variables|Default|GetSpline))
  (bind _returnvalue (Spline|GetSplineLength _spline))
  (bind _returnvalue_2 (/ _returnvalue _pipelength))
  (bind _returnvalue_3 (Math|Float|Truncate _returnvalue_2))
  (for _index (range 0 (- _returnvalue_3 1))
    (if (Utilities|IsValid (Utilities|Array|Get(acopy) (Variables|Default|GetsplineMeshComponents) _index))
      (SplineMesh|SetStartandEnd (Utilities|Array|Get(acopy) (Variables|Default|GetsplineMeshComponents) _index) (Spline|GetLocationatDistanceAlongSpline _spline_2 (* _index _pipelength) "Local") (Math|Vector|ClampVectorSize (Spline|GetTangentatDistanceAlongSpline _spline_2 (* _index _pipelength) "Local") 0.0 (Variables|Default|GetpipeLength)) (Spline|GetLocationatDistanceAlongSpline _spline_2 (* (+ _index 1) _pipelength) "Local") (Math|Vector|ClampVectorSize (Spline|GetTangentatDistanceAlongSpline _spline_2 (* (+ _index 1) _pipelength) "Local") 0.0 (Variables|Default|GetpipeLength)) true :!class /Script/Engine.SplineMeshComponent)
      (else
        (bind _returnvalue_4 (AddComponent|AddSplineMeshComponent false))
        (SplineMesh|SetForwardAxis _returnvalue_4 "Y" false)
        (Components|StaticMesh|SetStaticMesh _returnvalue_4 (Variables|Default|Getpipe))
        (SplineMesh|SetStartandEnd _returnvalue_4 (Spline|GetLocationatDistanceAlongSpline _spline_2 (* _index _pipelength) "Local") (Math|Vector|ClampVectorSize (Spline|GetTangentatDistanceAlongSpline _spline_2 (* _index _pipelength) "Local") 0.0 (Variables|Default|GetpipeLength)) (Spline|GetLocationatDistanceAlongSpline _spline_2 (* (+ _index 1) _pipelength) "Local") (Math|Vector|ClampVectorSize (Spline|GetTangentatDistanceAlongSpline _spline_2 (* (+ _index 1) _pipelength) "Local") 0.0 (Variables|Default|GetpipeLength)) true :!class /Script/Engine.SplineMeshComponent)
        (Collision|SetCollisionEnabled _returnvalue_4 "QueryAndPhysics")
        (Utilities|Array|SetArrayElem (Variables|Default|GetsplineMeshComponents) _index _returnvalue_4 true))))
  (Math|Integer|CompareInt (Utilities|Array|Length (Variables|Default|GetsplineMeshComponents)) _returnvalue_3
    (:>
      (for _index_2 (range _returnvalue_3 (Utilities|Array|Length (Variables|Default|GetsplineMeshComponents)))
        (Utilities|IsValid (Utilities|Array|Get(acopy) (Variables|Default|GetsplineMeshComponents) _index_2)
          (:Is%20Valid
            (Components|DestroyComponent (Utilities|Array|Get(acopy) (Variables|Default|GetsplineMeshComponents) _index_2))
            (Variables|Default|SetsplineMeshComponents (Utilities|Array|MakeArray 0))
            (for (_array_element _array_index) (Components|GetChildrenComponents (Variables|Default|GetSpline) false)
              (bind _asspline_mesh_component (Utilities|Casting|CastToSplineMeshComponent _array_element))
              (Utilities|Array|SetArrayElem (Variables|Default|GetsplineMeshComponents) _array_index _asspline_mesh_component true))))))))