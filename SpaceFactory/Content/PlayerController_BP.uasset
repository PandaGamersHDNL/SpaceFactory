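; Player controller that toggles a build mode, switching control between the player character and a builder pawn.
; On begin play it caches the player's pawn and spawns a builder pawn at build eye height.
; The BuildMode input possesses the builder pawn with a building menu and mouse cursor shown, or returns to the character, removing the menu and hiding the cursor.
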(event EventBeginPlay
  (Variables|Default|SetPlayerCharacter (Game|Player|GetPlayerPawn 0))
  (bind _returnvalue (Game|SpawnActorfromClass "/Game/BuilderPawn_BP.BuilderPawn_BP_C" (Math|Transform|MakeTransform (Math|Vector|MakeVector 0.0 0.0 (Variables|Default|GetBuildEyeHeight))) "AlwaysSpawn" 0 0))
  (Variables|Default|SetBuilderPawn _returnvalue))

(event EventTick
  (params (DeltaSeconds :type Float%20%28single-precision%29)))

(event Input|ActionEvents|InputActionBuildMode
  (params (Key :type Key%20Structure :default "None"))
  (:Pressed
    (bind _output_get (Variables|Default|SetBuildMode? (not (Variables|Default|GetBuildMode?))))
    (if _output_get
      (Pawn|Possess (Variables|Default|GetBuilderPawn))
      (bind _returnvalue (UserInterface|CreateWidget "/Game/BuildingMenu.BuildingMenu_C"))
      (UserInterface|Viewport|AddtoViewport _returnvalue 0)
      (Variables|Default|SetbShowMouseCursor true)
      (else
        (Pawn|Possess (Variables|Default|GetPlayerCharacter))
        (Widget|RemovefromParent _returnvalue)
        (Variables|Default|SetbShowMouseCursor false)))))

(fn ConstructionScript)