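; A pneumatic tube Blueprint that bends a spline mesh along one segment of its spline.
; Every Tick, it sets the mesh's start and end from the locations and tangents at Point and the following point, in local space.
; The construction script enables query and physics collision on the mesh.
; An unconnected branch, which never runs, would create an overlap-only spline mesh and fit it using world-space coordinates.
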(event EventBeginPlay)

(event EventTick
  (params (DeltaSeconds :type Float%20%28single-precision%29))
  (bind _spline (Variables|Default|GetSpline))
  (bind _point (Variables|Default|Getpoint))
  (bind _point_2 (Variables|Default|Getpoint))
  (bind (_location _tangent) (Spline|GetLocationandTangentatSplinePoint _spline _point "Local"))
  (bind _returnvalue (+ _point_2 1))
  (bind (_location_2 _tangent_2) (Spline|GetLocationandTangentatSplinePoint _spline _returnvalue "Local"))
  (SplineMesh|SetStartandEnd (Variables|Default|GetSplineMesh) _location _tangent _location_2 _tangent_2 true :!class /Script/Engine.SplineMeshComponent))

(fn ConstructionScript
  (Collision|SetCollisionEnabled (Variables|Default|GetSplineMesh) "QueryAndPhysics"))